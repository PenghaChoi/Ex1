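; BP_CountBox is a counter in the collect game that shows a running count on a TextRender component.
; The DoGet event takes an IsFruit1 flag, adds one to Count for fruit or subtracts one otherwise, then updates the text.
; AddCount only prints a debug string and does not change the count.
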(event EventDoGet
  (params (IsFruit1 :type Boolean))
  (if IsFruit1
    (Variables|Default|SetCount (+ (Variables|Default|GetCount) 1))
    (else
      (Variables|Default|SetCount (- (Variables|Default|GetCount) 1))))
  (Rendering|Components|TextRender|SetText (Variables|Default|GetTextRender) (Utilities|Text|ToText(Integer) (Variables|Default|GetCount))))

(fn ConstructionScript)

(fn AddCount
  (Development|PrintString "AddCount"))